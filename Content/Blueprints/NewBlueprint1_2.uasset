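; Interactable lever actor that, on Interact, tilts its lever and slides a static mesh along X.
; Any actor overlap enables player 0's input on it, plays a sound and adds a Press prompt widget; nothing here reverses this.
; Two Interact press handlers set Open, which is never read here, and each play a timeline, one driving lever pitch, the other mesh position.
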(event Collision|EventActorBeginOverlap
  (params (OtherActor :type Actor%20Object%20Reference))
  (Input|EnableInput (Game|GetPlayerController 0))
  (Audio|PlaySoundatLocation "/Engine/EditorSounds/GamePreview/EjectFromPlayer.EjectFromPlayer" (Transformation|GetActorLocation) "0, 0, 0" 1.0 1.0 0.0 0 0 0)
  ;[1 1 1] f
  (bind _returnvalue (UserInterface|CreateWidget "/Game/widgets/press.press_C"))
  (UserInterface|Viewport|AddtoViewport _returnvalue 0))

(event Input|ActionEvents|InputActionInteract
  (params (Key :type Key%20Structure :default "None"))
  (:Pressed
    (Variables|Default|Setopen true)
    (bind _newtrack_0 (Timeline|Timeline_0 Play)
      (:Update
        (Transformation|SetRelativeRotation (Variables|Default|Getlever_Box002) (Math|Rotator|MakeRotator 9e+01 _newtrack_0 -3.6e+02) false false)))))

(event Input|ActionEvents|InputActionInteract
  (params (Key :type Key%20Structure :default "None"))
  (:Pressed
    (Variables|Default|Setopen true)
    (bind _newtrack (Timeline|Timeline_1 Play)
      (:Update
        (Transformation|SetRelativeLocation (Variables|Default|GetStaticMesh) (Math|Vector|MakeVector _newtrack -1.24e+03 0.0) false false)))))

(fn ConstructionScript)