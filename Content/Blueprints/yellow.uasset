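; Explosive actor that detonates when shot by a FirstPersonProjectile and deals heavy damage to any Character that overlaps it.
; A projectile hit on the Hhh component spawns an explosion effect there and destroys the Hhh and Box components.
; The actor then destroys itself when that effect ends play.
; A Character overlap instead sends a take-damage message, destroys the actor immediately and plays a 2D explosion sound.
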(event OnComponentHit(hhh)
  (params (HitComponent :type Primitive%20Component%20Object%20Reference) (OtherActor :type Actor%20Object%20Reference) (OtherComp :type Primitive%20Component%20Object%20Reference) (NormalImpulse :type Vector :default "0, 0, 0") (Hit :type Hit%20Result%20Structure%20%28by%20ref%29))
  ;[1 1 1] only destroy if get hit
  (Utilities|Casting|CastToFirstPersonProjectile OtherActor)
  (Utilities|FlowControl|Sequence
    (:then_0
      (bind _returnvalue (Game|SpawnActorfromClass "/Game/StarterContent/Blueprints/Blueprint_Effect_Explosion.Blueprint_Effect_Explosion_C" (Transformation|GetWorldTransform (Variables|Default|Gethhh)) "Undefined" 0 0))
      (Variables|Default|SetfireExplotion _returnvalue))
    (:then_1
      (Components|DestroyComponent (Variables|Default|Gethhh)))))

(event OnEndPlay(fireExplotion)
  (params (Actor :type Actor%20Object%20Reference) (EndPlayReason :type EEndPlayReason%20Enum :default "Destroyed"))
  (Actor|DestroyActor))

(event Collision|EventActorBeginOverlap
  (params (OtherActor :type Actor%20Object%20Reference))
  ;[1 1 1] taking hit
  (Utilities|Casting|CastToCharacter OtherActor)
  (Class|Damage|Takedamage(Message) OtherActor 500)
  (Actor|DestroyActor)
  (Audio|PlaySound2D "/Game/StarterContent/Audio/Explosion01.Explosion01" 1.0 1.0 0.0 0 0))

(fn ConstructionScript)