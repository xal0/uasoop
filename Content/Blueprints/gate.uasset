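; Gate actor that the player operates with the Interact input after walking into it.
; Overlap by the FirstPersonCharacter enables input on the actor, plays a sound and adds a Press widget to the viewport.
; Two Interact release handlers each clear the Open flag and play a timeline, UpDown moving one mesh along Z and Push moving the other along X.
; Nothing here disables input or removes the widget afterwards.
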(event Collision|EventActorBeginOverlap
  (params (OtherActor :type Actor%20Object%20Reference))
  (Utilities|Casting|CastToFirstPersonCharacter OtherActor)
  (Input|EnableInput (Game|GetPlayerController 0))
  (Audio|PlaySoundatLocation "/Engine/EditorSounds/GamePreview/EjectFromPlayer.EjectFromPlayer" (Transformation|GetActorLocation) "0, 0, 0" 1.0 1.0 0.0 0 0 0)
  ;[1 1 1] f
  (bind _returnvalue (UserInterface|CreateWidget "/Game/widgets/press.press_C"))
  (UserInterface|Viewport|AddtoViewport _returnvalue 0))

(event Input|ActionEvents|InputActionInteract
  (params (Key :type Key%20Structure :default "None"))
  (:Released
    (if true
      (Variables|Default|Setopen false)
      (bind _newtrack_0 (Timeline|up%20down Play)
        (:Update
          (Transformation|SetRelativeLocation (Variables|Default|GetStaticMesh) (Math|Vector|MakeVector 0.0 0.0 _newtrack_0) false false))))))

(event Input|ActionEvents|InputActionInteract
  (params (Key :type Key%20Structure :default "None"))
  (:Released
    (if true
      (Variables|Default|Setopen false)
      (bind _newtrack_0 (Timeline|push Play)
        (:Update
          (Transformation|SetRelativeLocation (Variables|Default|GetStaticMesh1) (Math|Vector|MakeVector _newtrack_0 2.857142 -2e+01) false false))))))

(fn ConstructionScript)